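; Lamp pickup in Horror Engine that gives the player the flashlight as main equipment.
; It can be inspected, and taken directly or from inspection when Takeable, through a shared DoOnce that shows an "added to equipment" notice.
; It writes its mesh and inspection settings to the player's save inventory cache.
; On retake it restores those settings and silently re-equips the flashlight.
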(event Custom|CustomEvent_2
  (params (InventorySave :type Inventory%20Save%20Structure))
  (bind (_meshsettings _inspectionsettings) (Utilities|Struct|BreakInventorySave InventorySave))
  ;[1 1 1] Retake
  (Variables|Default|SetMeshSettings _meshsettings)
  (Variables|Default|SetInspectionSettings _inspectionsettings)
  (CallFunction|SetMesh (Variables|Default|GetCylinder) (Variables|Default|GetMeshSettings))
  (CallFunction|SetInspection (Variables|Default|GetInspectionSettings))
  (Variables|Default|SetTakeSound 0)
  (CallFunction|Take true true false)
  (bind _asmaster (CallFunction|GetPlayer))
  (Default|TakeFlashlight _asmaster))

(event Custom|CustomEvent_3
  ;[1 1 1] AddToSaveCache
  (bind _asmaster (CallFunction|GetPlayer))
  (Utilities|Array|Add (Variables|/Game/HorrorEngine/Blueprints/Core/HE_SaveGameComponent.HE_SaveGameComponent_C|GetInventoryCache (Variables|/Game/HorrorEngine/HorrorEngine.HorrorEngine_C|GetHE_SaveGameComponent _asmaster)) (Utilities|Struct|MakeInventorySave "NewEnumerator7" (Variables|Default|GetMeshSettings) (Variables|Default|GetInspectionSettings) false)))

(event Custom|CustomEvent
  (params (HorrorEvent :type Boolean))
  ;[1 1 1] Inspection Settings
  (if (not HorrorEvent)
    (CallFunction|BeginInspection)))

(event Custom|CustomEvent_1
  (params (HorrorEvent :type Boolean))
  ;[1 1 1] Take Settings
  (if (Variables|Default|GetTakeable)
    (Utilities|FlowControl|DoOnce false
      (:Completed
        (CallFunction|Take true false false)
        (bind _asmaster (CallFunction|GetPlayer))
        (Default|TakeFlashlight _asmaster)
        (CallFunction|Notice "" (Variables|Default|GetItemName) "added to equipment.")))
    (else
      (CallFunction|AlternativeUse HorrorEvent))))

(event EventInspectionAlternativeUse
  ;[1 1 1] Inspection Settings
  (CallFunction|EndInspection false))

(event EventInspectionUse
  ;[1 1 1] Take Settings
  (if (Variables|Default|GetTakeable)
    (Utilities|FlowControl|DoOnce false
      (:Completed
        (CallFunction|Take true false false)
        (bind _asmaster (CallFunction|GetPlayer))
        (Default|TakeFlashlight _asmaster)
        (CallFunction|Notice "" (Variables|Default|GetItemName) "added to equipment.")))))

(fn ConstructionScript
  (|CallParentFunction))