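; BP_Wheel is a spinnable wheel for the Horror Engine combination lock.
; SpinWheel passes a DoOnce gate and plays a timeline that writes WheelRotation to the mesh yaw.
; On finish it adds the timeline's Alpha to WheelRotation, calls NumberCheck, reopens the gate and wraps the angle to zero at a full turn.
; NumberCheck and RandomizeWheel are empty here.
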(event Custom|SpinWheel
  (Utilities|FlowControl|DoOnce false
    (:Completed
      (bind _alpha (Timeline|Timeline_0 PlayFromStart)
        (:Update
          (Transformation|SetRelativeRotation (Variables|Default|GetWheelMesh) (Math|Rotator|MakeRotator 0.0 0.0 (Variables|Default|GetWheelRotation)) false false))
        (:Finished
          (Variables|Default|SetWheelRotation (+ (Variables|Default|GetWheelRotation) _alpha))
          (CallFunction|NumberCheck)
          (CallFunction|SpinWheelReset)
          (if (>= (Variables|Default|GetWheelRotation) 3.6e+02)
            (Variables|Default|SetWheelRotation 0.0)))))))

(event Custom|SpinWheelReset
  (Utilities|FlowControl|DoOnce false) ; enters at Reset
)

(fn ConstructionScript)

(fn NumberCheck)

(fn RandomizeWheel)