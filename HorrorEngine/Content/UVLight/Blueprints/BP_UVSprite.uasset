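; A decal sprite that reacts to nearby UV emitters, driving its material's intensity and projection position.
; Construction sizes the detection sphere and decal and creates a dynamic material with color, texture, noise, projection and seeded random offset.
; Each tick it sums distance-falloff strength from overlapping BI_UVEmit actors.
; A proximity-weighted direction sum, projected onto the actor's forward-normal plane, becomes the material's X/Y offset.
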(event EventTick
  (params (DeltaSeconds :type Float%20%28single-precision%29))
  (CallFunction|CalculateUV))

(fn ConstructionScript
  (Components|Sphere|SetSphereRadius (Variables|Default|GetSphere) (Variables|Base|GetRadius) true)
  (bind _returnvalue (Rendering|Material|CreateDynamicMaterialInstance (Variables|Default|GetDecal) :!class /Script/Engine.DecalComponent))
  (bind _output_get (Variables|Default|SetMaterial _returnvalue))
  (Rendering|Material|SetScalarParameterValue _output_get "RandomOffset" (Math|Random|RandomFloatfromStream (Variables|Noise|GetRandomSeed)) :!class /Script/Engine.MaterialInstanceDynamic)
  (Rendering|Material|SetTextureParameterValue (Variables|Default|GetMaterial) "Texture" (Variables|Base|GetTexture))
  (Rendering|Material|SetVectorParameterValue (Variables|Default|GetMaterial) "Color" (Variables|Base|GetColor) :!class /Script/Engine.MaterialInstanceDynamic)
  (Rendering|Material|SetScalarParameterValue (Variables|Default|GetMaterial) "NoisePow" (Variables|Noise|GetNoisePow) :!class /Script/Engine.MaterialInstanceDynamic)
  (Rendering|Material|SetScalarParameterValue (Variables|Default|GetMaterial) "NoiseU" (Variables|Noise|GetNoiseV) :!class /Script/Engine.MaterialInstanceDynamic)
  (Rendering|Material|SetScalarParameterValue (Variables|Default|GetMaterial) "NoiseV" (Variables|Noise|GetNoiseU) :!class /Script/Engine.MaterialInstanceDynamic)
  (Rendering|Material|SetScalarParameterValue (Variables|Default|GetMaterial) "ProjectRadius" (Variables|Projection|GetProjectSize) :!class /Script/Engine.MaterialInstanceDynamic)
  (Rendering|Material|SetScalarParameterValue (Variables|Default|GetMaterial) "ProjectMult" (Variables|Projection|GetProjectIntensity) :!class /Script/Engine.MaterialInstanceDynamic)
  (Rendering|Material|SetScalarParameterValue (Variables|Default|GetMaterial) "ProjectDensity" (- 1.0 (Variables|Projection|GetProjectFalloff)) :!class /Script/Engine.MaterialInstanceDynamic)
  (Transformation|SetWorldScale3D (Variables|Default|GetDecal) (Variables|Base|GetDecalScale)))

(fn CalculateUV
  (bind _material (Variables|Default|GetMaterial))
  (Utilities|FlowControl|Sequence
    (:then_0
      (LocalVariables|SetStrengthSum 0.0)
      (LocalVariables|SetVectorSum "0, 0, 0"))
    (:then_1
      (for _array_element (Collision|GetOverlappingActors (Variables|Default|GetSphere) "/Script/Engine.Actor" :!class /Script/Engine.PrimitiveComponent)
        (if (Utilities|DoesObjectImplementInterface _array_element "/Game/UVLight/Blueprints/BI_UVEmit.BI_UVEmit_C")
          (bind (_location _strength) (Class|BIUVEmit|GetUV(Message) _array_element (Transformation|GetWorldLocation (Variables|Default|GetDecal))))
          (LocalVariables|SetStrengthSum (+ (* (Math|Float|Power (- 1.0 (/ (Math|Vector|VectorLength (- _location (Transformation|GetWorldLocation (Variables|Default|GetDecal)))) (Variables|Base|GetRadius))) (Variables|Base|GetDistanceExponent)) _strength) (LocalVariables|GetStrengthSum)))
          (LocalVariables|SetVectorSum (+ (LocalVariables|GetVectorSum) (* (Math|Vector|Normalize (- _location (Transformation|GetWorldLocation (Variables|Default|GetDecal)))) (- (Variables|Base|GetRadius) (Math|Vector|VectorLength (- _location (Transformation|GetWorldLocation (Variables|Default|GetDecal))))))))))
      (Rendering|Material|SetScalarParameterValue _material "Intensity" (LocalVariables|GetStrengthSum) :!class /Script/Engine.MaterialInstanceDynamic)
      (Rendering|Material|SetScalarParameterValue _material "X" (+ 0.5 (.Y (Math|Vector2D|BreakVector2D (* (Math|Vector2D|Normalize2D (Math|Vector2D|MakeVector2D (* (Math|Vector|DotProduct (Math|Vector|Normalize (Class|KismetMathLibrary|ProjectPointontoPlane (LocalVariables|GetVectorSum) "0, 0, 0" (Transformation|GetActorForwardVector))) (Transformation|GetActorUpVector)) (Math|Vector|VectorLength (Class|KismetMathLibrary|ProjectPointontoPlane (LocalVariables|GetVectorSum) "0, 0, 0" (Transformation|GetActorForwardVector))) -1.0) (* (Math|Vector|VectorLength (Class|KismetMathLibrary|ProjectPointontoPlane (LocalVariables|GetVectorSum) "0, 0, 0" (Transformation|GetActorForwardVector))) (Math|Vector|DotProduct (Math|Vector|Normalize (Class|KismetMathLibrary|ProjectPointontoPlane (LocalVariables|GetVectorSum) "0, 0, 0" (Transformation|GetActorForwardVector))) (Transformation|GetActorRightVector))))) (Math|Float|Power (/ (Math|Vector|VectorLength (LocalVariables|GetVectorSum)) (Variables|Base|GetRadius)) (Variables|Projection|GetProjectExponent)))))) :!class /Script/Engine.MaterialInstanceDynamic)
      (Rendering|Material|SetScalarParameterValue _material "Y" (+ 0.5 (.X (Math|Vector2D|BreakVector2D (* (Math|Vector2D|Normalize2D (Math|Vector2D|MakeVector2D (* (Math|Vector|DotProduct (Math|Vector|Normalize (Class|KismetMathLibrary|ProjectPointontoPlane (LocalVariables|GetVectorSum) "0, 0, 0" (Transformation|GetActorForwardVector))) (Transformation|GetActorUpVector)) (Math|Vector|VectorLength (Class|KismetMathLibrary|ProjectPointontoPlane (LocalVariables|GetVectorSum) "0, 0, 0" (Transformation|GetActorForwardVector))) -1.0) (* (Math|Vector|VectorLength (Class|KismetMathLibrary|ProjectPointontoPlane (LocalVariables|GetVectorSum) "0, 0, 0" (Transformation|GetActorForwardVector))) (Math|Vector|DotProduct (Math|Vector|Normalize (Class|KismetMathLibrary|ProjectPointontoPlane (LocalVariables|GetVectorSum) "0, 0, 0" (Transformation|GetActorForwardVector))) (Transformation|GetActorRightVector))))) (Math|Float|Power (/ (Math|Vector|VectorLength (LocalVariables|GetVectorSum)) (Variables|Base|GetRadius)) (Variables|Projection|GetProjectExponent)))))) :!class /Script/Engine.MaterialInstanceDynamic))))