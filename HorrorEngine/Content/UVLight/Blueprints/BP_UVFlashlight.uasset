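; UV flashlight actor that reports how strongly its SpotLight beam affects a given target point.
; GetUV returns the point on the beam axis at the target's distance, along with a strength value.
; Strength combines linear distance falloff over 512 units with a dot-product cone test, remapped from the Precision threshold and scaled by the Strength variable.
; All logic lives in that query, as the events and construction script are empty.
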(event EventBeginPlay)

(event Collision|EventActorBeginOverlap
  (params (OtherActor :type Actor%20Object%20Reference)))

(event EventTick
  (params (DeltaSeconds :type Float%20%28single-precision%29)))

(fn ConstructionScript)

(fn GetUV
  (params (Target :type Vector :default "0, 0, 0"))
  (bind _spotlight (Variables|Default|GetSpotLight))
  (bind _returnvalue (Transformation|GetWorldLocation _spotlight))
  (bind _returnvalue_2 (- Target _returnvalue))
  (bind _returnvalue_3 (Math|Vector|VectorLength _returnvalue_2))
  (return (+ (Transformation|GetWorldLocation (Variables|Default|GetSpotLight)) (* (Math|Vector|GetForwardVector (Variables|Default|GetSpotLight)) _returnvalue_3)) (* (Math|Float|Max(Float) (- 1.0 (/ _returnvalue_3 512.0)) 0.0) (Math|Float|MapRangeClamped (Math|Vector|DotProduct (Math|Vector|Normalize _returnvalue_2) (Math|Vector|GetForwardVector (Variables|Default|GetSpotLight))) (Variables|Default|GetPrecision) 1.0 0.0 (Variables|Default|GetStrength)))))